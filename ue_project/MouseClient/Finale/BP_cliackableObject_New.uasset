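; Clickable actor that reports left and right mouse clicks on itself to a server through a VR mouse client reference.
; On click, it deprojects the viewport mouse position and uses the resulting world position, not a hit point, labeling any non-left button as right.
; HandleClick normalizes each axis against hardcoded ranges, calls SendWorldClickEvent and prints whether sending succeeded.
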(event EventBeginPlay)

(event Collision|EventActorBeginOverlap
  (params (OtherActor :type Actor%20Object%20Reference)))

(event EventTick
  (params (DeltaSeconds :type Float%20%28single-precision%29)))

(event MouseInput|EventActorOnClicked
  (params (ButtonPressed :type Key%20Structure :default "None"))
  (bind _mouseclient_ref (Variables|Default|GetMouseClient_Ref))
  (Development|PrintString "Hello")
  (bind _returnvalue (Class|WidgetLayoutLibrary|GetMousePositiononViewport))
  (if (== ButtonPressed "LeftMouseButton")
    (Development|PrintString "Hello")
    (CallFunction|HandleClick "left button down" (.WorldPosition (Class|GameplayStatics|DeprojectScreentoWorld (Game|GetPlayerController 0) _returnvalue)) _mouseclient_ref)
    (Development|PrintString "left button down")
    (else
      (CallFunction|HandleClick "right button down" (.WorldPosition (Class|GameplayStatics|DeprojectScreentoWorld (Game|GetPlayerController 0) _returnvalue)) _mouseclient_ref)
      (Development|PrintString "right button down"))))

(fn ConstructionScript)

(fn HandleClick
  (params (EventType :type String) (ClickLocation :type Vector) (VRMouseClient_Ref :type VR%20Mouse%20Client%20Object%20Reference))
  (bind (_x _y _z) (Math|Vector|BreakVector ClickLocation))
  (bind _returnvalue (Class|VRMouseClient|SendWorldClickEvent VRMouseClient_Ref EventType (Math|Float|NormalizetoRange _x -1.2e+03 1.92e+03) (Math|Float|NormalizetoRange _y -2e+02 1.08e+03) (Math|Float|NormalizetoRange _z 81.0 2e+02)))
  (if _returnvalue
    (Development|PrintString "Sent to server")
    (else
      (Development|PrintString "Failed to send"))))